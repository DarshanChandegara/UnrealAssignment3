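; BP_BuilderController is a builder controller Blueprint that manages an on-screen widget for notification messages.
; A CreateWidget event creates the widget, stores a reference to it, adds it to the viewport and hides its notification text.
; A Notify event shows the given message in that text, then hides it after a short delay.
; BeginPlay and Tick are unused, so both events rely on being called.
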(event `self.CreateWidget`
  (bind _returnvalue (`|CreateWidget` "/Game/Blueprint/MyWidget.MyWidget_C"))
  (bind _output_get (set `self.MyWidgetRef` _returnvalue))
  (`UserWidget.AddToViewport` _output_get 0)
  (`Widget.SetVisibility` (`/Game/Blueprint/MyWidget.NotificationText` _output_get) "Hidden"))

(event `self.Notify`
  (params (message :type String))
  (bind _notificationtext (`/Game/Blueprint/MyWidget.NotificationText` (`self.MyWidgetRef`)))
  (`Widget.SetVisibility` _notificationtext "Visible")
  (set `TextBlock.Text` (`KismetTextLibrary.Conv_StringToText` message) _notificationtext)
  (`KismetSystemLibrary.Delay` 2.0)
  (set `Widget.Visibility` "Hidden" _notificationtext))

(fn `UserConstructionScript`)